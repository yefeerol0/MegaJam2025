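; Interactable actor that runs a needle-and-zone skill check QTE, raising the score and destroying itself on completion.
; Box overlap enables Interact, which locks pawn input and starts the challenge on the MJQTESkillCheck component.
; Tick spins the widget's needle toward a randomized success zone, with timed repeats until enough hits.
; A missed press or three full turns without input triggers the GameMode's lose condition.
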(event `HandleChallengeSuccess`
  (bind _widgetref (`self.WidgetRef`))
  (bind _playerref (`self.PlayerRef`))
  (`self.EnableInput` (`Controller.K2_GetPawn` _playerref) _playerref)
  (`/Engine/EditorBlueprintResources/StandardMacros.IsValid` _widgetref
    (:`Is Valid`
      (`Widget.RemoveFromParent` _widgetref))
    (:`Is Not Valid`
      _))
  (`/Game/Kaan/MJB_GameMode.Manager_IncreaseScore` (`self.GameMode`))
  (`self.K2_DestroyActor`))

(event `self.ReceiveBeginPlay`
  (bind _mj_qte_skillcheck (`self.MJ_QTE_SkillCheck`))
  (set `self.GameMode` (cast `/Game/Kaan/MJB_GameMode` (`GameplayStatics.GetGameMode`) :!pure true))
  (add `MJ_QTE_SkillCheckComponent.OnSkillCheckInputPressed` _mj_qte_skillcheck (delegate `HandleInput`))
  (add `MJ_QTE_SkillCheckComponent.OnChallengeComplete` _mj_qte_skillcheck (delegate `HandleChallengeSuccess`)))

(event `HandleInput`
  (bind _mj_qte_skillcheck (`self.MJ_QTE_SkillCheck`))
  (bind _returnvalue (mod (- (`self.CurrentNeedleAngle`) (`self.SuccessZoneStart`)) 360.0))
  (if (`self.bIsSkillCheckActive`)
    (set `self.bIsSkillCheckActive` false)
    (set `self.bWasSuccess` false)
    (if (and (>= _returnvalue (`self.ZoneVisualOffset`)) (<= _returnvalue (+ (`self.ZoneVisualOffset`) (`self.ZoneWidth`))))
      (set `self.bWasSuccess` true)
      (`MJ_QTE_SkillCheckComponent.ReportSkillCheckResult` (`self.MJ_QTE_SkillCheck`) (`self.bWasSuccess`))
      (`/Engine/EditorBlueprintResources/StandardMacros.IsValid` (`self.MJ_QTE_SkillCheck`)
        (:`Is Valid`
          (if (not (== (`MJ_QTE_SkillCheckComponent.SuccessesRequired` _mj_qte_skillcheck) (`MJ_QTE_SkillCheckComponent.CurrentSuccessCount` _mj_qte_skillcheck)))
            (bind _returnvalue_2 (`KismetSystemLibrary.K2_SetTimerDelegate` (delegate `TriggerNewSkillCheck`) 1.0))
            (set `self.SkillCheckTimerHandle` _returnvalue_2))))
      (else
        (`/Game/Kaan/MJB_GameMode.LoseCondition` (`self.GameMode`))))))

(event `self.Box.OnComponentBeginOverlap`
  (params (OverlappedComponent :type "PrimitiveComponent Object Reference") (OtherActor :type "Actor Object Reference") (OtherComp :type "PrimitiveComponent Object Reference") (OtherBodyIndex :type Integer) (bFromSweep :type Boolean) (SweepResult :type "HitResult Structure (by ref)"))
  (bind _asmjb_player_character (cast `/Game/Blueprints/MJB_PlayerCharacter` OtherActor))
  (bind _asplayer_controller (cast `PlayerController` (`Pawn.GetController` _asmjb_player_character)))
  (bind _output_get (set `self.PlayerRef` _asplayer_controller))
  (`self.EnableInput` _output_get))

(event `self.Box.OnComponentEndOverlap`
  (params (OverlappedComponent :type "PrimitiveComponent Object Reference") (OtherActor :type "Actor Object Reference") (OtherComp :type "PrimitiveComponent Object Reference") (OtherBodyIndex :type Integer))
  (bind _widgetref (`self.WidgetRef`))
  (bind _asmjb_player_character (cast `/Game/Blueprints/MJB_PlayerCharacter` OtherActor))
  (bind _asplayer_controller (cast `PlayerController` (`Pawn.GetController` _asmjb_player_character)))
  (`self.DisableInput` (`self.PlayerRef`) _asplayer_controller)
  (`KismetSystemLibrary.K2_ClearAndInvalidateTimerHandle` (`self.SkillCheckTimerHandle`))
  (set `self.bIsSkillCheckActive` false)
  (`/Engine/EditorBlueprintResources/StandardMacros.IsValid` _widgetref
    (:`Is Valid`
      (`Widget.RemoveFromParent` _widgetref)
      (`MJ_QTE_SkillCheckComponent.StopChallenge` (`self.MJ_QTE_SkillCheck`)))))

(event `InputAction|Interact`
  (params (Key :type "Key Structure"))
  (bind _playerref (`self.PlayerRef`))
  (:`Pressed`
    (`/Engine/EditorBlueprintResources/StandardMacros.DoOnce` false
      (:`Completed`
        (`self.DisableInput` (`Controller.K2_GetPawn` _playerref) _playerref)
        (`MJ_QTE_SkillCheckComponent.StartChallenge` (`self.MJ_QTE_SkillCheck`) (`self.PlayerRef`))
        (`self.TriggerNewSkillCheck`)))))

(event `TriggerNewSkillCheck`
  (bind _widgetref (`self.WidgetRef`))
  (`/Engine/EditorBlueprintResources/StandardMacros.IsValid` _widgetref
    (:`Is Valid`
      (`Widget.RemoveFromParent` _widgetref))
    (:`Is Not Valid`
      _))
  (set `self.bIsSkillCheckActive` true)
  (set `self.CurrentNeedleAngle` 0.0)
  (bind _output_get (set `self.SuccessZoneStart` (`KismetMathLibrary.RandomFloatInRange` 90.0 270.0)))
  (set `self.SuccessZoneEnd` (+ _output_get 40.0))
  (bind _returnvalue (`|CreateWidget` "/Game/Blueprints/MJ_WBP_QTE_SkillCheck.MJ_WBP_QTE_SkillCheck_C"))
  (bind _output_get_2 (set `self.WidgetRef` _returnvalue))
  (`/Game/Blueprints/MJ_WBP_QTE_SkillCheck.SetupZone` _output_get_2 _output_get)
  (`UserWidget.AddToViewport` (`self.WidgetRef`) 0))

(event `self.ReceiveTick`
  (params (DeltaSeconds :type "Float (single-precision)"))
  (if (`self.bIsSkillCheckActive`)
    (bind _output_get (set `self.CurrentNeedleAngle` (+ (`self.CurrentNeedleAngle`) (* (`self.NeedleSpeed`) DeltaSeconds))))
    (`/Game/Blueprints/MJ_WBP_QTE_SkillCheck.UpdateNeedle` (`self.WidgetRef`) _output_get)
    (if (> (`self.CurrentNeedleAngle`) 1080.0)
      (set `self.bIsSkillCheckActive` false)
      (`Widget.RemoveFromParent` (`self.WidgetRef`))
      (`MJ_QTE_SkillCheckComponent.ReportSkillCheckResult` (`self.MJ_QTE_SkillCheck`) false)
      (`/Game/Kaan/MJB_GameMode.LoseCondition` (`self.GameMode`)))))

(fn `UserConstructionScript`)