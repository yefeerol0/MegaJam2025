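; Script paper actor that slides into place when spawned and drops away when the player turns it off.
; On BeginPlay it binds to the player character's TurnOffScriptEvent, plays an opening sound and runs the rise timeline.
; That event plays a closing sound and runs the fall timeline, then destroys the actor.
; Both timelines add their value to the paper's current relative Z each update, so movement accumulates rather than following absolute positions.
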(event `self.ReceiveBeginPlay`
  (bind _scriptpaper (`self.ScriptPaper`))
  (bind (_relativelocation_x _relativelocation_y _relativelocation_z) (`KismetMathLibrary.BreakVector` (`SceneComponent.RelativeLocation` _scriptpaper)))
  (bind _asmjb_player_character (cast `/Game/Blueprints/MJB_PlayerCharacter` (`GameplayStatics.GetPlayerCharacter` 0)))
  (add `/Game/Blueprints/MJB_PlayerCharacter.TurnOffScriptEvent` _asmjb_player_character (delegate `TurnOffScriptEvent_Event`))
  (`GameplayStatics.PlaySound2D` "/Game/SFX/Kagit_Acma.Kagit_Acma" 1.0 1.0 0.0 null null)
  (bind (_direction _1) (`Timeline|ScriptPaperRise`)
    (:`Update`
      (`SceneComponent.K2_SetRelativeLocation` _scriptpaper (`KismetMathLibrary.MakeVector` _relativelocation_x _relativelocation_y (+ _relativelocation_z _1)) false false))))

(event `TurnOffScriptEvent_Event`
  (bind _scriptpaper (`self.ScriptPaper`))
  (bind (_relativelocation_x _relativelocation_y _relativelocation_z) (`KismetMathLibrary.BreakVector` (`SceneComponent.RelativeLocation` _scriptpaper)))
  (`GameplayStatics.PlaySound2D` "/Game/SFX/Kagit_Kapama.Kagit_Kapama" 1.0 1.0 0.0 null null)
  (bind (_direction _1) (`Timeline|ScriptPaperFall`)
    (:`Update`
      (`SceneComponent.K2_SetRelativeLocation` _scriptpaper (`KismetMathLibrary.MakeVector` _relativelocation_x _relativelocation_y (+ _relativelocation_z _1)) false false))
    (:`Finished`
      (`self.K2_DestroyActor`))))

(fn `UserConstructionScript`)