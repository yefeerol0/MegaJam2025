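; Interactable QTE cube that starts a button-mash quick time event and destroys itself on success.
; Entering the box collision as the player character enables input on the actor, and leaving disables it.
; The first Interact press creates a progress bar widget and starts the QTE mash component with the player controller.
; Tick feeds the component's progress to the widget, which is removed on success.
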(event `self.ReceiveTick`
  (params (DeltaSeconds :type "Float (single-precision)"))
  (bind _widgetref (`self.WidgetRef`))
  (`/Engine/EditorBlueprintResources/StandardMacros.IsValid` _widgetref
    (:`Is Valid`
      (`/Game/Blueprints/MJ_WBP_QTEBar.UpdateProgress` _widgetref (`MJ_QTEMashComponent.CurrentProgress` (`self.MJ_QTEMash`))))))

(event `self.QTEBoxCollision.OnComponentBeginOverlap`
  (params (OverlappedComponent :type "PrimitiveComponent Object Reference") (OtherActor :type "Actor Object Reference") (OtherComp :type "PrimitiveComponent Object Reference") (OtherBodyIndex :type Integer) (bFromSweep :type Boolean) (SweepResult :type "HitResult Structure (by ref)"))
  (bind _asmjb_player_character (cast `/Game/Blueprints/MJB_PlayerCharacter` OtherActor))
  (bind _asplayer_controller (cast `PlayerController` (`Pawn.GetController` _asmjb_player_character)))
  (bind _output_get (set `self.PlayerRef` _asplayer_controller))
  (`self.EnableInput` _output_get))

(event `self.QTEBoxCollision.OnComponentEndOverlap`
  (params (OverlappedComponent :type "PrimitiveComponent Object Reference") (OtherActor :type "Actor Object Reference") (OtherComp :type "PrimitiveComponent Object Reference") (OtherBodyIndex :type Integer))
  (bind _asmjb_player_character (cast `/Game/Blueprints/MJB_PlayerCharacter` OtherActor))
  (bind _asplayer_controller (cast `PlayerController` (`Pawn.GetController` _asmjb_player_character)))
  (`self.DisableInput` _asplayer_controller)
  (set `self.PlayerRef` null))

(event `self.MJ_QTEMash.OnQTESuccess`
  (`Widget.RemoveFromParent` (`self.WidgetRef`))
  (`self.K2_DestroyActor`))

(event `InputAction|Interact`
  (params (Key :type "Key Structure"))
  (:`Pressed`
    (`/Engine/EditorBlueprintResources/StandardMacros.DoOnce` false
      (:`Completed`
        (bind _returnvalue (`|CreateWidget` "/Game/Blueprints/MJ_WBP_QTEBar.MJ_WBP_QTEBar_C"))
        (bind _output_get (set `self.WidgetRef` _returnvalue))
        (`UserWidget.AddToViewport` _output_get 0)
        (bind _output_get_2 (set `self.MJ_QTEMash` (`self.MJ_QTEMash`)))
        (`MJ_QTEMashComponent.StartQTE` _output_get_2 (`self.PlayerRef`))))))

(fn `UserConstructionScript`)