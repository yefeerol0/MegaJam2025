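; MJ_ObjectivePoint is a world objective marker that triggers the player's dialogue screen when its detection volume is first overlapped.
; On BeginPlay it caches the MJB_PlayerCharacter.
; The first DetectPlayer overlap, not filtered by actor and gated by DoOnce, switches the floor circle and beam to green materials.
; It then calls TurnOnDialogueScreen on the character, passing itself and a player orientation rotation.
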(event `self.ReceiveBeginPlay`
  (bind _asmjb_player_character (cast `/Game/Blueprints/MJB_PlayerCharacter` (`GameplayStatics.GetPlayerCharacter` 0)))
  (set `self.CharacterRef` _asmjb_player_character))

(event `self.DetectPlayer.OnComponentBeginOverlap`
  (params (OverlappedComponent :type "PrimitiveComponent Object Reference") (OtherActor :type "Actor Object Reference") (OtherComp :type "PrimitiveComponent Object Reference") (OtherBodyIndex :type Integer) (bFromSweep :type Boolean) (SweepResult :type "HitResult Structure (by ref)"))
  (`/Engine/EditorBlueprintResources/StandardMacros.DoOnce` false
    (:`Completed`
      (`PrimitiveComponent.SetMaterial` (`self.FloorCircle`) 0 "/Game/Blueprints/DialogueSystem/Materials/M_ObjectiveGreen.M_ObjectiveGreen")
      (`PrimitiveComponent.SetMaterial` (`self.ObjectiveBeam`) 0 "/Game/Blueprints/DialogueSystem/Materials/M_ObjectiveBeamGreen.M_ObjectiveBeamGreen")
      (`/Game/Blueprints/MJB_PlayerCharacter.TurnOnDialogueScreen` (`self.CharacterRef`) self (`self.PlayerOrientation`)))))

(fn `UserConstructionScript`)