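; Actor component on a Character that tracks whether the owner stands on a target spot and gates throwing and dropping accordingly.
; It binds to MJB_KaanGameMode events on BeginPlay and answers checks through the game mode: throw is available only on a spot, drop only off it.
; Stepping onto a spot stores it and its target and disables movement; hitting the target clears both and restores walking.
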(event `self.ReceiveBeginPlay`
  (set `self.OwnerChar` (cast `Character` (`self.GetOwner`) :!pure true))
  (set `self.GameMode` (cast `/Game/Kaan/MJB_KaanGameMode` (`GameplayStatics.GetGameMode`) :!pure true))
  (set `self.CurrentTargetStop` null)
  (set `self.CurrentTarget` null)
  (set `self.IsOnTargetSpot` false)
  (add `/Game/Kaan/MJB_KaanGameMode.Throw_SpotCheck` (`self.GameMode`) (delegate `Throw_IsOnTargetSpotCheck`))
  (add `/Game/Kaan/MJB_KaanGameMode.HitTheTarget` (`self.GameMode`) (delegate `HitTheTarget_Event`))
  (add `/Game/Kaan/MJB_KaanGameMode.Drop_SpotCheck` (`self.GameMode`) (delegate `Drop_SpotCheck_Event`))
  (add `/Game/Kaan/MJB_KaanGameMode.TargetSpot_Available` (`self.GameMode`) (delegate `TargetSpotAvailable_Event`)))

(event `HitTheTarget_Event`
  (params (HitTarget :type "/Game/Kaan/MJB_Target Object Reference"))
  (`KismetSystemLibrary.PrintString` "Hello")
  (set `self.CurrentTarget` null)
  (set `self.CurrentTargetStop` null)
  (`CharacterMovementComponent.SetMovementMode` (`Character.CharacterMovement` (`self.OwnerChar`)) "MOVE_Walking" 0)
  (set `self.IsOnTargetSpot` false))

(event `Drop_SpotCheck_Event`
  (bind _gamemode (`self.GameMode`))
  (if (`self.IsOnTargetSpot`)
    (`/Game/Kaan/MJB_KaanGameMode.Drop_NotAvailable` _gamemode)
    (else
      (`/Game/Kaan/MJB_KaanGameMode.Drop_Available` _gamemode))))

(event `Throw_IsOnTargetSpotCheck`
  (bind _gamemode (`self.GameMode`))
  (if (`self.IsOnTargetSpot`)
    (`/Game/Kaan/MJB_KaanGameMode.Throw_Available` _gamemode)
    (else
      (`/Game/Kaan/MJB_KaanGameMode.Throw_NotAvailable` _gamemode))))

(event `TargetSpotAvailable_Event`
  (params (SteppedTargetSpot :type "/Game/Kaan/MJB_TargetStop Object Reference"))
  (bind _output_get (set `self.CurrentTargetStop` SteppedTargetSpot))
  (set `self.CurrentTarget` (`/Game/Kaan/MJB_TargetStop.MyTarget` _output_get))
  (`CharacterMovementComponent.DisableMovement` (`Character.CharacterMovement` (`self.OwnerChar`)))
  (set `self.IsOnTargetSpot` true))