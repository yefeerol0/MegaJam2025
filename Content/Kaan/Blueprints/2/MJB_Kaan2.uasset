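; MJB_Kaan2 is a player character Blueprint handling movement-based camera shake, item pickup and closing a script.
; Every Tick it starts an idle, walk or sprint camera shake, chosen by velocity and CanJump.
; Overlapping an actor that implements BPI_Throwable2 sends it a pickup message with the character as argument.
; The TurnOffScript input fires a turn-off event, then clears IsScriptOpen after a short delay.
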(event `Camera Shake`
  (`self.InitializeShake`))

(event `self.ReceiveTick`
  (params (DeltaSeconds :type "Float (single-precision)"))
  (`self.Camera Shake`))

(event `InputAction|TurnOffScript`
  (params (Key :type "Key Structure"))
  (:`Pressed`
    (`self.TurnOffScriptEvent`)
    (`KismetSystemLibrary.Delay` 1.0)
    (set `self.IsScriptOpen` false)))

(event `self.ReceiveActorBeginOverlap`
  (params (OtherActor :type "Actor Object Reference"))
  (if (`KismetSystemLibrary.DoesImplementInterface` OtherActor "/Game/Kaan/Blueprints/2/BPI_Throwable2.BPI_Throwable2_C")
    (message `/Game/Kaan/Blueprints/2/BPI_Throwable2.PickUp` OtherActor self)))

(fn `InitializeShake`
  (bind _returnvalue (`GameplayStatics.GetPlayerController` 0))
  (bind _returnvalue_2 (`KismetMathLibrary.VSize` (`self.GetVelocity`)))
  (if (and (> _returnvalue_2 0.0) (`self.CanJump`))
    (if (< _returnvalue_2 800.0)
      (`PlayerController.ClientStartCameraShake` :`self` _returnvalue :`Shake` "/Game/Blueprints/CameraShakes/CS_Walk.CS_Walk_C")
      (else
        (`PlayerController.ClientStartCameraShake` :`self` _returnvalue :`Shake` "/Game/Blueprints/CameraShakes/CS_Sprint.CS_Sprint_C")))
    (else
      (`PlayerController.ClientStartCameraShake` :`self` _returnvalue :`Shake` "/Game/Blueprints/CameraShakes/CS_Idle.CS_Idle_C"))))

(fn `UserConstructionScript`)