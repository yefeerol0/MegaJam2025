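; MJB_Throwable2 is a throwable object that a picker can grab and carry at its mesh's RightBallSocket.
; PickUp turns off collision and physics on ThrowableMesh, then attaches to the socket, snapping location and keeping world rotation and scale.
; It then adds AttachOffset and AttachRotation to the resulting world location and rotation, so the offsets are not socket-relative.
; Aim and Throw events are empty stubs.
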(event `/Game/Kaan/Blueprints/2/BPI_Throwable2.PickUp`
  (params (Picker :type "Character Object Reference"))
  (bind (_returnvalue_roll _returnvalue_pitch _returnvalue_yaw) (`KismetMathLibrary.BreakRotator` (`self.K2_GetActorRotation`)))
  (bind (_attachrotation_roll _attachrotation_pitch _attachrotation_yaw) (`KismetMathLibrary.BreakRotator` (`self.AttachRotation`)))
  (bind _throwablemesh (`self.ThrowableMesh`))
  (`PrimitiveComponent.SetCollisionProfileName` _throwablemesh "NoCollision" true)
  (`PrimitiveComponent.SetSimulatePhysics` _throwablemesh false)
  (`self.K2_AttachToComponent` (`Character.Mesh` Picker) "RightBallSocket" "SnapToTarget" "KeepWorld" "KeepWorld")
  (`self.K2_SetActorLocation` (+ (`self.K2_GetActorLocation`) (`self.AttachOffset`)))
  (`self.K2_SetActorRotation` (`KismetMathLibrary.MakeRotator` (+ _returnvalue_roll _attachrotation_roll) (+ _returnvalue_pitch _attachrotation_pitch) (+ _returnvalue_yaw _attachrotation_yaw))))

(event `/Game/Kaan/Blueprints/2/BPI_Throwable2.Aim`)

(event `/Game/Kaan/Blueprints/2/BPI_Throwable2.Throw`)

(fn `UserConstructionScript`)