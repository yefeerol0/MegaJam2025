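; Player character with movement-based camera shake and a throwable ball that has an aim preview.
; Each tick picks idle, walk or sprint shake from velocity and CanJump.
; Holding E runs a looping timer that rebuilds spline meshes along a predicted projectile path; release clears them and launches MJB_Throwable with the same camera-derived velocity, remapping pitch for lift.
; TurnOffScript input fires an event, then clears IsScriptOpen after a delay.
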(event `Camera Shake`
  (`self.InitializeShake`))

(event `self.ReceiveTick`
  (params (DeltaSeconds :type "Float (single-precision)"))
  (`self.Camera Shake`))

(event `InputAction|TurnOffScript`
  (params (Key :type "Key Structure"))
  (:`Pressed`
    (`self.TurnOffScriptEvent`)
    (`KismetSystemLibrary.Delay` 1.0)
    (set `self.IsScriptOpen` false)))

(event `Key|E`
  (params (Key :type "Key Structure"))
  (bind _returnvalue (`KismetMathLibrary.GetForwardVector` (`PlayerCameraManager.GetCameraRotation` (`GameplayStatics.GetPlayerCameraManager` 0))))
  (bind (_returnvalue_x _returnvalue_y) (`KismetMathLibrary.BreakVector` (* _returnvalue 1000.0)))
  (:`Pressed`
    (`StaticMeshComponent.SetStaticMesh` (`self.Throwable`) "/Engine/VREditor/BasicMeshes/SM_Ball_01.SM_Ball_01")
    (`self.DrawProjectileWay`))
  (:`Released`
    (`KismetSystemLibrary.K2_ClearAndInvalidateTimerHandle` (`self.ProjectilePathTimer`))
    (`self.ClearSplineWay`)
    (`StaticMeshComponent.SetStaticMesh` (`self.Throwable`) null)
    (bind _returnvalue_2 (`|SpawnActorFromClass` "/Game/Kaan/Blueprints/MJB_Throwable.MJB_Throwable_C" (`KismetMathLibrary.MakeTransform` (`SceneComponent.K2_GetComponentLocation` (`self.Throwable`))) "Undefined" "MultiplyWithRoot" null null))
    (`PrimitiveComponent.AddImpulse` (`/Game/Kaan/Blueprints/MJB_Throwable.Ball` _returnvalue_2) (`KismetMathLibrary.MakeVector` _returnvalue_x _returnvalue_y (* (`KismetMathLibrary.MapRangeUnclamped` (.z _returnvalue) 0.0 1.0 3.0 10.0) 150.0)) "None" true)))

(event `Key|LeftMouseButton`
  (params (Key :type "Key Structure")))

(event `DrawProjectileWay`
  (bind _returnvalue (`KismetSystemLibrary.K2_SetTimerDelegate` (delegate `UpdateProjectileWay`) 0.01 true))
  (set `self.ProjectilePathTimer` _returnvalue))

(event `UpdateProjectileWay`
  (bind _projectilespline (`self.ProjectileSpline`))
  (bind _returnvalue (`KismetMathLibrary.GetForwardVector` (`PlayerCameraManager.GetCameraRotation` (`GameplayStatics.GetPlayerCameraManager` 0))))
  (bind (_returnvalue_x _returnvalue_y) (`KismetMathLibrary.BreakVector` (* _returnvalue 1000.0)))
  (`self.ClearSplineWay`)
  (bind _predictresult (`GameplayStatics.Blueprint_PredictProjectilePath_Advanced` (make `PredictProjectilePathParams` (`SceneComponent.K2_GetComponentLocation` (`self.Throwable`)) (`KismetMathLibrary.MakeVector` _returnvalue_x _returnvalue_y (* (`KismetMathLibrary.MapRangeUnclamped` (.z _returnvalue) 0.0 1.0 3.0 10.0) 150.0)) true 0.0 1.0 true "ECC_WorldStatic" _ (`|MakeArray` self :!type "Actor Object Reference") 13.0 0.0 "None" 5.0)))
  (for _array_element (`.PathData` (break `PredictProjectilePathResult` _predictresult))
    (`SplineComponent.AddSplinePoint` (`self.ProjectileSpline`) (`.Location` (break `PredictProjectilePathPointData` _array_element)) "World" true))
  (for _index (range 1 (+ (`SplineComponent.GetNumberOfSplinePoints` (`self.ProjectileSpline`)) 1))
    (bind _returnvalue_2 (`AddComponent|NODE_AddSplineMeshComponent-0` :`bManualAttachment` true))
    (`KismetArrayLibrary.Array_Add` (`self.SplineMesh`) _returnvalue_2)
    (bind (_location _tangent) (`SplineComponent.GetLocationAndTangentAtSplinePoint` _projectilespline _index "World"))
    (bind (_location_2 _tangent_2) (`SplineComponent.GetLocationAndTangentAtSplinePoint` _projectilespline (+ _index 1) "World"))
    (`SplineMeshComponent.SetStartAndEnd` _returnvalue_2 _location _tangent (`KismetMathLibrary.VLerp` _location _location_2 0.5) (`KismetMathLibrary.VLerp` _tangent _tangent_2 0.5) true)))

(event `ClearSplineWay`
  (bind _splinemesh (`self.SplineMesh`))
  (`ActorComponent.K2_DestroyComponent` _splinemesh)
  (`KismetArrayLibrary.Array_Clear` _splinemesh)
  (`SplineComponent.ClearSplinePoints` (`self.ProjectileSpline`) true))

(fn `InitializeShake`
  (bind _returnvalue (`GameplayStatics.GetPlayerController` 0))
  (bind _returnvalue_2 (`KismetMathLibrary.VSize` (`self.GetVelocity`)))
  (if (and (> _returnvalue_2 0.0) (`self.CanJump`))
    (if (< _returnvalue_2 800.0)
      (`PlayerController.ClientStartCameraShake` :`self` _returnvalue :`Shake` "/Game/Blueprints/CameraShakes/CS_Walk.CS_Walk_C")
      (else
        (`PlayerController.ClientStartCameraShake` :`self` _returnvalue :`Shake` "/Game/Blueprints/CameraShakes/CS_Sprint.CS_Sprint_C")))
    (else
      (`PlayerController.ClientStartCameraShake` :`self` _returnvalue :`Shake` "/Game/Blueprints/CameraShakes/CS_Idle.CS_Idle_C"))))

(fn `UserConstructionScript`)