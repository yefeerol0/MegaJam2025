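; Character component for picking up, dropping and throwing physics pickups held at a mesh socket.
; Holding left mouse oscillates throw power on a sine wave and draws a timer-driven debug path prediction; right mouse drops.
; Releasing requests a GameMode spot check, whose available and not-available events are both bound to the throw.
; Launch velocity blends camera aim, per-item arc and inherited horizontal movement, with pawn collision ignored during a cooldown.
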(event `self.ReceiveBeginPlay`
  (set `self.OwnerChar` (cast `Character` (`self.GetOwner`) :!pure true))
  (bind _output_get (set `self.GameMode` (cast `/Game/Kaan/MJB_KaanGameMode` (`GameplayStatics.GetGameMode`) :!pure true)))
  (set `self.PickedUpActor` null)
  (set `self.IsJustThrowed` false)
  (add `/Game/Kaan/MJB_KaanGameMode.Throw_Available` _output_get (delegate `ThrowAvailable`))
  (add `/Game/Kaan/MJB_KaanGameMode.Throw_NotAvailable` _output_get (delegate `ThrowAvailable`)))

(event `ThrowAvailable`
  (`self.Throw`))

(event `Key|RightMouseButton`
  (params (Key :type "Key Structure"))
  (bind _pickedupactor (`self.PickedUpActor`))
  (:`Released`
    (if (not (`self.IsJustThrowed`))
      (`/Engine/EditorBlueprintResources/StandardMacros.IsValid` _pickedupactor
        (:`Is Valid`
          (`self.DropDown` _pickedupactor))
        (:`Is Not Valid`
          (`KismetSystemLibrary.PrintString` "Nothing to drop down"))))))

(event `Key|LeftMouseButton`
  (params (Key :type "Key Structure"))
  (:`Pressed`
    (if (not (`self.IsJustThrowed`))
      (`/Engine/EditorBlueprintResources/StandardMacros.IsValid` (`self.PickedUpActor`)
        (:`Is Valid`
          (`self.Aim`))
        (:`Is Not Valid`
          (`KismetSystemLibrary.PrintString` "No object in hand")))))
  (:`Released`
    (if (not (`self.IsJustThrowed`))
      (`/Engine/EditorBlueprintResources/StandardMacros.IsValid` (`self.PickedUpActor`)
        (:`Is Valid`
          (if (`self.IsAiming`)
            (`/Game/Kaan/MJB_KaanGameMode.Throw_SpotCheck` (`self.GameMode`))
            (else
              (`KismetSystemLibrary.PrintString` "You can't shoot without aim"))))
        (:`Is Not Valid`
          (`KismetSystemLibrary.PrintString` "No object in hand"))))))

(event `self.ReceiveTick`
  (params (DeltaSeconds :type "Float (single-precision)"))
  (if (`self.IsCharging`)
    (bind _output_get (set `self.PowerAlpha` (+ (* (`KismetMathLibrary.Sin` (`KismetSystemLibrary.MakeLiteralDouble` (* (`KismetSystemLibrary.MakeLiteralDouble` (- (`KismetSystemLibrary.GetGameTimeInSeconds`) (`self.ChargeStartTime`))) (`self.ChargeFreq`) (`KismetMathLibrary.GetPI`) 2.0))) 0.5) 0.5)))
    (set `self.CurrentThrowSpeed` (`KismetMathLibrary.Lerp` (`self.MinThrowSpeed`) (`self.MaxThrowSpeed`) _output_get))))

(event `Throw`
  (bind _pickupmesh (`/Game/Kaan/MJB_Pickup.PickupMesh` (`self.PickedUpActor`)))
  (bind _pickupmesh_2 (`/Game/Kaan/MJB_Pickup.PickupMesh` (`self.PickedUpActor`)))
  (set `self.IsJustThrowed` true)
  (set `self.IsCharging` false)
  (set `self.IsAiming` false)
  (`KismetSystemLibrary.K2_ClearAndInvalidateTimerHandle` (`self.DrawProjectileEvent`))
  (`SceneComponent.K2_DetachFromComponent` _pickupmesh_2 "KeepWorld" "KeepWorld" "KeepWorld" true)
  (`PrimitiveComponent.SetCollisionProfileName` _pickupmesh_2 "PickupIgnorePawn" true)
  (`PrimitiveComponent.SetSimulatePhysics` _pickupmesh_2 true)
  (bind _finalvelocity (`self.CalculateVelocity` (`self.InheritScale`)))
  (`PrimitiveComponent.SetPhysicsLinearVelocity` _pickupmesh _finalvelocity false "None")
  (`KismetSystemLibrary.Delay` (`self.NextPickupCooldown`))
  (`PrimitiveComponent.SetCollisionProfileName` _pickupmesh "Pickup" true)
  (set `/Game/Kaan/MJB_Pickup.IsBeingThrowed` true (`self.PickedUpActor`))
  (set `self.PickedUpActor` null)
  (set `self.IsJustThrowed` false))

(event `DrawProjectileWay`
  (bind _returnvalue (`KismetSystemLibrary.K2_SetTimerDelegate` (delegate `UpdateProjectileWay`) 0.01 true))
  (set `self.DrawProjectileEvent` _returnvalue))

(event `UpdateProjectileWay`
  (bind _finalvelocity (`self.CalculateVelocity` (`self.InheritScale`)))
  (`GameplayStatics.Blueprint_PredictProjectilePath_Advanced` (make `PredictProjectilePathParams` (`SceneComponent.K2_GetComponentLocation` (`/Game/Kaan/MJB_Pickup.PickupMesh` (`self.PickedUpActor`))) _finalvelocity true 0.0 2.0 true "ECC_WorldStatic" _ (`|MakeArray` (`self.OwnerChar`) :!type "Actor Object Reference") 60.0 -980.0 "ForOneFrame" 5.0)))

(fn `Aim`
  (set `self.IsCharging` true)
  (set `self.ChargeStartTime` (`KismetSystemLibrary.GetGameTimeInSeconds`))
  (`self.DrawProjectileWay`)
  (set `self.IsAiming` true))

(fn `CalculateVelocity`
  (params (CharSpeedInheritRatio :type "Float (double-precision)"))
  (returns (finalVelocity :type "Vector Structure"))
  (bind _returnvalue (`PlayerCameraManager.GetCameraRotation` (`GameplayStatics.GetPlayerCameraManager` 0)))
  (bind (_velocity_x _velocity_y) (`KismetMathLibrary.BreakVector` (`MovementComponent.Velocity` (`Character.CharacterMovement` (`self.OwnerChar`)))))
  (return (+ (* (`KismetMathLibrary.Normal` (+ (* (`KismetMathLibrary.GetUpVector` _returnvalue) (`/Game/Kaan/MJB_Pickup.ArcFactor` (`self.PickedUpActor`))) (`KismetMathLibrary.GetForwardVector` _returnvalue))) (`self.CurrentThrowSpeed`)) (* (`KismetMathLibrary.MakeVector` _velocity_x _velocity_y) (`self.InheritScale`)))))

(fn `DropDown`
  (params (ItemInHand :type "/Game/Kaan/MJB_Pickup Object Reference"))
  (bind _pickupmesh (`/Game/Kaan/MJB_Pickup.PickupMesh` ItemInHand))
  (bind _drawprojectileevent (`self.DrawProjectileEvent`))
  (`SceneComponent.K2_DetachFromComponent` _pickupmesh "KeepWorld" "KeepWorld" "KeepWorld" true)
  (`PrimitiveComponent.SetCollisionProfileName` _pickupmesh "Pickup" true)
  (`PrimitiveComponent.SetSimulatePhysics` _pickupmesh true)
  (set `self.PickedUpActor` null)
  (if (`KismetSystemLibrary.K2_IsValidTimerHandle` _drawprojectileevent)
    (`KismetSystemLibrary.K2_ClearAndInvalidateTimerHandle` _drawprojectileevent)))

(fn `PickUp`
  (params (ItemToPickUp :type "/Game/Kaan/MJB_Pickup Object Reference"))
  (returns (PickUpSuccsessful :type Boolean))
  (locals (localPickup :type "/Game/Kaan/MJB_Pickup Object Reference"))
  (bind _localpickup (`local.localPickup`))
  (bind _localpickup_2 (`local.localPickup`))
  (bind _pickupmesh (`/Game/Kaan/MJB_Pickup.PickupMesh` _localpickup))
  (bind _pickupmesh_2 (`/Game/Kaan/MJB_Pickup.PickupMesh` _localpickup_2))
  (`/Engine/EditorBlueprintResources/StandardMacros.IsValid` (`self.PickedUpActor`)
    (:`Is Valid`
      (return false))
    (:`Is Not Valid`
      (bind _output_get (set `local.localPickup` ItemToPickUp))
      (bind _pickupmesh_3 (`/Game/Kaan/MJB_Pickup.PickupMesh` _output_get))
      (`PrimitiveComponent.SetSimulatePhysics` _pickupmesh_3 false)
      (`PrimitiveComponent.SetCollisionProfileName` _pickupmesh_3 "NoCollision" true)
      (bind _returnvalue (`SceneComponent.K2_AttachToComponent` _pickupmesh_3 (`Character.Mesh` (`self.OwnerChar`)) "PickupSlot" "SnapToTarget" "SnapToTarget" "KeepWorld" true))
      (if _returnvalue
        (`SceneComponent.K2_SetRelativeLocation` _pickupmesh (+ (`SceneComponent.RelativeLocation` _pickupmesh) (`/Game/Kaan/MJB_Pickup.AttachOffset` _localpickup)) false false)
        (`SceneComponent.K2_SetRelativeRotation` _pickupmesh_2 (`self.AddRotator` (`SceneComponent.RelativeRotation` _pickupmesh_2) (`/Game/Kaan/MJB_Pickup.AttachRotation` _localpickup_2)) false false)
        (bind _output_get_2 (set `self.PickedUpActor` (`local.localPickup`)))
        (set `/Game/Kaan/MJB_Pickup.IsBeingThrowed` false _output_get_2)
        (return true)
        (else
          (return false))))))